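; ChoppedElementBP is a chopped item that the player can pick up, carry, drop and place on counters.
; OnCarry enables input when the character's hands are free, and X then fixes the item and registers it on the ThirdPersonCharacter.
; Tick teleports it above the carrier or assigned counter instead of attaching it.
; Drop restores gravity and clears the carry state, while IsSomethingPlacedOnElement always returns false.
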(event `self.ReceiveTick`
  (params (DeltaSeconds :type "Float (single-precision)"))
  (bind _ispositionfixated (`self.isPositionFixated`))
  (`|ExecutionSequence`
    (:`then_1`
      (if (and (`self.isCarried`) _ispositionfixated)
        (`self.K2_SetActorLocation` (`KismetMathLibrary.MakeVector` (.x (`self.K2_GetActorLocation` (`self.carryActorReference`))) (.y (`self.K2_GetActorLocation` (`self.carryActorReference`))) (+ (.z (`self.K2_GetActorLocation` (`self.carryActorReference`))) 250.0)))
        (`self.DisableInput` (`GameplayStatics.GetPlayerController` 0))
        (elif _ispositionfixated
          (`self.K2_SetActorLocation` (`KismetMathLibrary.MakeVector` (.x (`self.K2_GetActorLocation` (`self.placedCounterReference`))) (.y (`self.K2_GetActorLocation` (`self.placedCounterReference`))) (+ (.z (`self.K2_GetActorLocation` (`self.placedCounterReference`))) 250.0))))))))

(event `Key|X`
  (params (Key :type "Key Structure"))
  (:`Pressed`
    (set `self.isPositionFixated` true)
    (`PrimitiveComponent.SetEnableGravity` (`self.Cylinder`) false)
    (bind _asthird_person_character (cast `/Game/ThirdPersonBP/Blueprints/ThirdPersonCharacter` (`self.carryActorReference`)))
    (set `/Game/ThirdPersonBP/Blueprints/ThirdPersonCharacter.isCarrying` true _asthird_person_character)
    (set `/Game/ThirdPersonBP/Blueprints/ThirdPersonCharacter.carryingObject` self _asthird_person_character)))

(event `/Game/CarryInterface.onCarry`
  (params (isCarried :type Boolean) (carryActor :type "Actor Object Reference"))
  (if isCarried
    (bind _output_get (set `self.carryActorReference` carryActor))
    (bind _asthird_person_character (cast `/Game/ThirdPersonBP/Blueprints/ThirdPersonCharacter` _output_get))
    (if (not (`/Game/ThirdPersonBP/Blueprints/ThirdPersonCharacter.isCarrying` _asthird_person_character))
      (`self.EnableInput` (`GameplayStatics.GetPlayerController` 0))
      (set `self.isCarried` true))
    (else
      (set `self.carryActorReference` null))))

(event `/Game/CarryInterface.drop`
  (params (carryActor :type "Actor Object Reference"))
  (bind _asthird_person_character (cast `/Game/ThirdPersonBP/Blueprints/ThirdPersonCharacter` carryActor))
  (set `/Game/ThirdPersonBP/Blueprints/ThirdPersonCharacter.isCarrying` false _asthird_person_character)
  (`PrimitiveComponent.SetEnableGravity` (`self.Cylinder`) true)
  (set `self.isPositionFixated` false)
  (set `self.isCarried` false))

(event `self.ReceiveBeginPlay`
  (set `self.isPositionFixated` true))

(event `/Game/CarryInterface.updatedCarriedElementForCounterPlace`
  (params (placedCounterReference :type "Actor Object Reference"))
  (set `self.isCarried` false)
  (set `self.isPositionFixated` true)
  (set `self.placedCounterReference` placedCounterReference))

(fn `isSomethingPlacedOnElement`
  (returns (isSomethingPlaced :type Boolean))
  (return false))

(fn `UserConstructionScript`)