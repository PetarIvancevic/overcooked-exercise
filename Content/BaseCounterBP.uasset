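; Base counter Blueprint where a third-person character can set down and pick up a single carried element, such as an onion.
; Placing clears the character's carry state, stores the element and notifies it by message, re-setting its location with zero offset.
; Taking hands the element back through a carry message, but is blocked for an onion once any chops are done.
; IsSomethingPlacedOnElement always returns false here.
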(event `/Game/CarryInterface.onCounterPlace`
  (params (carryActor :type "Actor Object Reference") (carriedActor :type "Actor Object Reference") (placeElement :type "Actor Object Reference"))
  (if (not (`self.isCarryingElement`))
    (bind _asthird_person_character (cast `/Game/ThirdPersonBP/Blueprints/ThirdPersonCharacter` carryActor))
    (set `/Game/ThirdPersonBP/Blueprints/ThirdPersonCharacter.isCarrying` false _asthird_person_character)
    (`self.K2_SetActorLocation` carriedActor (`KismetMathLibrary.MakeVector` (.x (`self.K2_GetActorLocation` carriedActor)) (.y (`self.K2_GetActorLocation` carriedActor)) (+ (.z (`self.K2_GetActorLocation` carriedActor)) 0.0)) false false)
    (set `self.isCarryingElement` true)
    (set `self.placedElement` carriedActor)
    (message `/Game/CarryInterface.updatedCarriedElementForCounterPlace` carriedActor self)))

(event `/Game/CarryInterface.takeFromCounter`
  (params (carryActor :type "Actor Object Reference"))
  (bind _placedelement (`self.placedElement`))
  (if (`self.isCarryingElement`)
    (bind _asonion_bp (cast `/Game/OnionBP` _placedelement)
      (:`then`
        (if (not (> (`/Game/OnionBP.numChopsDone` _asonion_bp) 0))
          (set `self.isCarryingElement` false :!label _label)
          (message `/Game/CarryInterface.onCarry` _placedelement true carryActor)
          (bind _asthird_person_character (cast `/Game/ThirdPersonBP/Blueprints/ThirdPersonCharacter` carryActor))
          (set `/Game/ThirdPersonBP/Blueprints/ThirdPersonCharacter.isCarrying` true _asthird_person_character)
          (set `/Game/ThirdPersonBP/Blueprints/ThirdPersonCharacter.carryingObject` (`self.placedElement`) _asthird_person_character)
          (set `self.placedElement` null)))
      (:`CastFailed`
        (goto _label)))))

(fn `isSomethingPlacedOnElement`
  (returns (isSomethingPlaced :type Boolean))
  (return false))

(fn `UserConstructionScript`)