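; Cooking counter that holds a cooking pot, accepts chopped elements from the player and drives the pot's cooking.
; Placing a pot, or adding an element to a pot with room, starts a looping cookChoppedElements timer on it by function name; adding also refreshes its progress bar.
; Taking the pot clears that timer and hands it to the character.
; OnInteract applies highlight materials, which Tick resets every frame.
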(event `/Game/InteractionInterface.OnInteract`
  (params (canCharacterInteract :type Boolean) (interactActor :type "Actor Object Reference"))
  (if canCharacterInteract
    (`|ExecutionSequence`
      (:`then_0`
        (`PrimitiveComponent.SetMaterial` (`self.CounterTop`) 0 "/Game/CounterElementRockMarbleOverlap.CounterElementRockMarbleOverlap"))
      (:`then_1`
        (`PrimitiveComponent.SetMaterial` (`self.CounterElement`) 0 "/Game/CounterWoodOverlap.CounterWoodOverlap")))))

(event `self.ReceiveTick`
  (params (DeltaSeconds :type "Float (single-precision)"))
  (`|ExecutionSequence`
    (:`then_0`
      (`PrimitiveComponent.SetMaterial` (`self.CounterTop`) 0 "/Game/StarterContent/Materials/M_Rock_Marble_Polished.M_Rock_Marble_Polished"))
    (:`then_1`
      (`PrimitiveComponent.SetMaterial` (`self.CounterElement`) 0 "/Game/CounterWoodNormal.CounterWoodNormal"))))

(event `self.ReceiveBeginPlay`
  (set `self.isCarryingElement` true))

(event `/Game/CarryInterface.takeFromCounter`
  (params (carryActor :type "Actor Object Reference"))
  (bind _placedelement (`self.placedElement`))
  (`KismetSystemLibrary.K2_ClearTimer` (`self.placedElement`) "cookChoppedElements")
  (bind _ascooking_pot_bp (cast `/Game/CookingPotBP` _placedelement))
  (set `/Game/CookingPotBP.carryActorReference` carryActor _ascooking_pot_bp)
  (set `/Game/CookingPotBP.carryCounterObject` null _ascooking_pot_bp)
  (set `self.isCarryingElement` false)
  (message `/Game/CarryInterface.onCarry` _placedelement true carryActor)
  (bind _asthird_person_character (cast `/Game/ThirdPersonBP/Blueprints/ThirdPersonCharacter` carryActor))
  (set `/Game/ThirdPersonBP/Blueprints/ThirdPersonCharacter.isCarrying` true _asthird_person_character)
  (set `/Game/ThirdPersonBP/Blueprints/ThirdPersonCharacter.carryingObject` (`self.placedElement`) _asthird_person_character)
  (set `self.placedElement` null))

(event `/Game/CarryInterface.onCounterPlace`
  (params (carryActor :type "Actor Object Reference") (carriedActor :type "Actor Object Reference") (placeElement :type "Actor Object Reference"))
  (if (`self.isCarryingElement`)
    (bind _aschopped_element_bp (cast `/Game/ChoppedElementBP` carriedActor))
    (bind _ascooking_pot_bp (cast `/Game/CookingPotBP` (`self.placedElement`)))
    (if (< (`/Game/CookingPotBP.numElementsInPot` _ascooking_pot_bp) 3)
      (`/Game/CookingPotBP.placeChoppedElementInPot` _ascooking_pot_bp _aschopped_element_bp)
      (`self.K2_DestroyActor` _aschopped_element_bp)
      (set `/Game/CookingPotBP.ovecookedTime` 0.0 _ascooking_pot_bp)
      (`ProgressBar.SetPercent` (`/Game/CookingPotBP.progressBarReference` _ascooking_pot_bp) (/ (`/Game/CookingPotBP.totalCookedNum` _ascooking_pot_bp) (* (`/Game/CookingPotBP.numElementsInPot` _ascooking_pot_bp) (`/Game/CookingPotBP.cookedElementNum` _ascooking_pot_bp))))
      (bind _asthird_person_character (cast `/Game/ThirdPersonBP/Blueprints/ThirdPersonCharacter` carryActor))
      (set `/Game/ThirdPersonBP/Blueprints/ThirdPersonCharacter.isCarrying` false _asthird_person_character)
      (set `/Game/ThirdPersonBP/Blueprints/ThirdPersonCharacter.carryingObject` null _asthird_person_character)
      (`KismetSystemLibrary.K2_ClearTimer` (`self.placedElement`) "cookChoppedElements")
      (`KismetSystemLibrary.K2_SetTimer` (`self.placedElement`) "cookChoppedElements" 1.0 true :!label _label))
    (else
      (cast `/Game/CookingPotBP` carriedActor)
      (bind _asthird_person_character_2 (cast `/Game/ThirdPersonBP/Blueprints/ThirdPersonCharacter` carryActor))
      (set `/Game/ThirdPersonBP/Blueprints/ThirdPersonCharacter.isCarrying` false _asthird_person_character_2)
      (`self.K2_SetActorLocation` carriedActor (`KismetMathLibrary.MakeVector` (.x (`self.K2_GetActorLocation` carriedActor)) (.y (`self.K2_GetActorLocation` carriedActor)) (+ (.z (`self.K2_GetActorLocation` carriedActor)) 0.0)) false false)
      (set `self.isCarryingElement` true)
      (set `self.placedElement` carriedActor)
      (message `/Game/CarryInterface.updatedCarriedElementForCounterPlace` carriedActor self)
      (goto _label))))

(fn `CheckIfReferencesAreEqual`
  (params (A :type "Object Object Reference") (B :type "Object Object Reference"))
  (if (== A B)
    _))

(fn `UserConstructionScript`)