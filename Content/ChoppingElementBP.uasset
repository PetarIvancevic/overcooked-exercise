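; Chopping counter Blueprint that lets the player chop an onion placed on it by holding C.
; A looping timer calls ChopIfElementExists, which advances chopping on the placed OnionBP while C is held.
; Once chopped, it spawns a fixed, gravity-free ChoppedElementBP at the onion's last transform as the new placed element.
; Interaction applies overlap highlight materials, which Tick resets every frame while also enabling input when carrying an element.
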(event `/Game/InteractionInterface.OnInteract`
  (params (canCharacterInteract :type Boolean) (interactActor :type "Actor Object Reference"))
  (if canCharacterInteract
    (`|ExecutionSequence`
      (:`then_0`
        (`PrimitiveComponent.SetMaterial` (`self.CounterTop`) 0 "/Game/CounterElementRockMarbleOverlap.CounterElementRockMarbleOverlap"))
      (:`then_1`
        (`PrimitiveComponent.SetMaterial` (`self.CounterElement`) 0 "/Game/CounterWoodOverlap.CounterWoodOverlap")))))

(event `self.ReceiveTick`
  (params (DeltaSeconds :type "Float (single-precision)"))
  (`|ExecutionSequence`
    (:`then_0`
      (`PrimitiveComponent.SetMaterial` (`self.CounterTop`) 0 "/Game/StarterContent/Materials/M_Rock_Marble_Polished.M_Rock_Marble_Polished"))
    (:`then_1`
      (`PrimitiveComponent.SetMaterial` (`self.CounterElement`) 0 "/Game/CounterWoodNormal.CounterWoodNormal"))
    (:`then_2`
      (if (`self.isCarryingElement`)
        (`self.EnableInput` (`GameplayStatics.GetPlayerController` 0))))))

(event `Key|C`
  (params (Key :type "Key Structure"))
  (:`Pressed`
    (set `self.isTryingToChop` true))
  (:`Released`
    (set `self.isTryingToChop` false)))

(event `self.ReceiveBeginPlay`
  (`KismetSystemLibrary.K2_SetTimer` null "chopIfElementExists" 0.3 true))

(fn `chopIfElementExists`
  (if (and (`self.isCarryingElement`) (`self.isTryingToChop`))
    (bind _asonion_bp (cast `/Game/OnionBP` (`self.placedElement`)))
    (if (not (`/Game/OnionBP.isChopped` _asonion_bp))
      (bind (_ischopped _lasttransform) (`/Game/OnionBP.chopOnion` _asonion_bp))
      (if _ischopped
        (bind _returnvalue (`|SpawnActorFromClass` "/Game/ChoppedElementBP.ChoppedElementBP_C" _lasttransform "AlwaysSpawn" "OverrideRootScale" null null))
        (set `/Game/ChoppedElementBP.placedCounterReference` self _returnvalue)
        (set `/Game/ChoppedElementBP.isPositionFixated` true _returnvalue)
        (set `self.placedElement` _returnvalue)
        (`PrimitiveComponent.SetEnableGravity` (`/Game/ChoppedElementBP.Cylinder` _returnvalue) false)))))

(fn `UserConstructionScript`
  (`parent.UserConstructionScript`))