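; Carryable cooking pot that takes chopped ingredients, shows up to three onion meshes and tracks their cooking.
; Tick pins the pot above its carrier or counter and projects its progress bar widget to screen space.
; Carry, drop and counter-placement events toggle input, gravity and the character's carrying state, with X confirming pickup.
; Externally called cook steps fill the bar by ingredient count, then accumulate overcook time, which the doneness check limits.
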(event `self.ReceiveTick`
  (params (DeltaSeconds :type "Float (single-precision)"))
  (bind _ispositionfixated (`self.isPositionFixated`))
  (`|ExecutionSequence`
    (:`then_0`
      (if (`KismetSystemLibrary.IsValid` (`self.progressBarReference`))
        (`UserWidget.SetPositionInViewport` (`self.progressBarWidget`) (`GameplayStatics.ProjectWorldToScreen` (`GameplayStatics.GetPlayerController` 0) (`SceneComponent.K2_GetComponentLocation` (`self.Cylinder`))) true)))
    (:`then_1`
      (if (and (`self.isCarried`) _ispositionfixated)
        (`self.K2_SetActorLocation` (`KismetMathLibrary.MakeVector` (.x (`self.K2_GetActorLocation` (`self.carryActorReference`))) (.y (`self.K2_GetActorLocation` (`self.carryActorReference`))) (+ (.z (`self.K2_GetActorLocation` (`self.carryActorReference`))) 250.0)))
        (`self.DisableInput` (`GameplayStatics.GetPlayerController` 0))
        (elif _ispositionfixated
          (`self.K2_SetActorLocation` (`KismetMathLibrary.MakeVector` (.x (`self.K2_GetActorLocation` (`self.carryCounterObject`))) (.y (`self.K2_GetActorLocation` (`self.carryCounterObject`))) (+ (.z (`self.K2_GetActorLocation` (`self.carryCounterObject`))) 250.0))))))))

(event `Key|X`
  (params (Key :type "Key Structure"))
  (:`Pressed`
    (set `self.isPositionFixated` true)
    (`PrimitiveComponent.SetEnableGravity` (`self.Cylinder`) false)
    (bind _asthird_person_character (cast `/Game/ThirdPersonBP/Blueprints/ThirdPersonCharacter` (`self.carryActorReference`)))
    (set `/Game/ThirdPersonBP/Blueprints/ThirdPersonCharacter.isCarrying` true _asthird_person_character)
    (set `/Game/ThirdPersonBP/Blueprints/ThirdPersonCharacter.carryingObject` self _asthird_person_character)))

(event `/Game/CarryInterface.onCarry`
  (params (isCarried :type Boolean) (carryActor :type "Actor Object Reference"))
  (if isCarried
    (bind _output_get (set `self.carryActorReference` carryActor))
    (bind _asthird_person_character (cast `/Game/ThirdPersonBP/Blueprints/ThirdPersonCharacter` _output_get))
    (if (not (`/Game/ThirdPersonBP/Blueprints/ThirdPersonCharacter.isCarrying` _asthird_person_character))
      (`self.EnableInput` (`GameplayStatics.GetPlayerController` 0))
      (set `self.isCarried` true))
    (else
      (set `self.carryActorReference` null))))

(event `self.ReceiveBeginPlay`
  (set `self.isPositionFixated` true)
  (`PrimitiveComponent.SetEnableGravity` (`self.Cylinder`) false))

(event `/Game/CarryInterface.drop`
  (params (carryActor :type "Actor Object Reference"))
  (bind _asthird_person_character (cast `/Game/ThirdPersonBP/Blueprints/ThirdPersonCharacter` carryActor))
  (set `/Game/ThirdPersonBP/Blueprints/ThirdPersonCharacter.isCarrying` false _asthird_person_character)
  (`PrimitiveComponent.SetEnableGravity` (`self.Cylinder`) true)
  (set `self.isPositionFixated` false)
  (set `self.isCarried` false))

(event `/Game/CarryInterface.updatedCarriedElementForCounterPlace`
  (params (placedCounterReference :type "Actor Object Reference"))
  (set `self.isCarried` false)
  (set `self.isPositionFixated` true)
  (set `self.carryCounterObject` placedCounterReference))

(fn `areChoppedElementsCooked`
  (returns (areCooked :type Boolean))
  (return (and (== (`self.numElementsInPot`) 3) (== (`self.totalCookedNum`) 300.0) (< (`self.ovecookedTime`) (`self.cookedElementNum`)))))

(fn `cookChoppedElements`
  (bind _totalcookednum (`self.totalCookedNum`))
  (if (> (`self.numElementsInPot`) 0)
    (if (== _totalcookednum 0.0)
      (bind _returnvalue (`|CreateWidget` "/Game/ProgressBarBP.ProgressBarBP_C" (`GameplayStatics.GetPlayerController` 0)))
      (bind _output_get (set `self.progressBarWidget` _returnvalue))
      (set `self.progressBarReference` (`/Game/ProgressBarBP.choppingProgressBar` _returnvalue))
      (`UserWidget.AddToViewport` _returnvalue 0)
      (`UserWidget.SetPositionInViewport` _output_get (100.0 100.0) true))
    (if (< _totalcookednum (* (`self.numElementsInPot`) (`self.cookedElementNum`)))
      (bind _output_get_2 (set `self.totalCookedNum` (+ (`self.cookedTimeIncreaseNum`) (`self.totalCookedNum`))))
      (`ProgressBar.SetPercent` (`self.progressBarReference`) (/ _output_get_2 (* (`self.numElementsInPot`) (`self.cookedElementNum`))))
      (else
        (set `self.ovecookedTime` (+ (`self.cookedTimeIncreaseNum`) (`self.ovecookedTime`)))))
    (else
      (`SceneComponent.SetVisibility` (`self.Onion03`) false false)
      (`SceneComponent.SetVisibility` (`self.Onion02`) false false)
      (`SceneComponent.SetVisibility` (`self.Onion01`) false false)
      (`Widget.RemoveFromParent` (`self.progressBarWidget`)))))

(fn `isSomethingPlacedOnElement`
  (returns (isSomethingPlaced :type Boolean))
  (return false))

(fn `placeChoppedElementInPot`
  (params (choppedElement :type "Actor Object Reference"))
  (cast `/Game/ChoppedElementBP` choppedElement)
  (set `self.numElementsInPot` (+ (`self.numElementsInPot`) 1))
  (`self.showProperNumElementsInPot`))

(fn `resetCookingSituation`
  (set `self.numElementsInPot` 0)
  (set `self.totalCookedNum` 0.0)
  (set `self.ovecookedTime` 0.0))

(fn `showProperNumElementsInPot`
  (bind _numelementsinpot (`self.numElementsInPot`))
  (if (== _numelementsinpot 1)
    (`SceneComponent.SetVisibility` (`self.Onion01`) true false)
    (elif (== _numelementsinpot 2)
      (`SceneComponent.SetVisibility` (`self.Onion02`) true false)
      (elif (== _numelementsinpot 3)
        (`SceneComponent.SetVisibility` (`self.Onion03`) true false)))))

(fn `UserConstructionScript`)