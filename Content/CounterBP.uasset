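; Counter actor that highlights itself with overlap materials when a character can interact with it.
; OnInteract swaps the top and base meshes to overlap materials, while Tick restores the normal marble and wood every frame, so the highlight depends on repeated interact calls.
; Helper graphs for reference-checked material swaps and toggling player input on overlap are defined but not called in the event graph.
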(event `/Game/InteractionInterface.OnInteract`
  (params (canCharacterInteract :type Boolean) (interactActor :type "Actor Object Reference"))
  (if canCharacterInteract
    (`|ExecutionSequence`
      (:`then_0`
        (`PrimitiveComponent.SetMaterial` (`self.CounterTop`) 0 "/Game/CounterElementRockMarbleOverlap.CounterElementRockMarbleOverlap"))
      (:`then_1`
        (`PrimitiveComponent.SetMaterial` (`self.CounterElement`) 0 "/Game/CounterWoodOverlap.CounterWoodOverlap")))))

(event `self.ReceiveTick`
  (params (DeltaSeconds :type "Float (single-precision)"))
  (`|ExecutionSequence`
    (:`then_0`
      (`PrimitiveComponent.SetMaterial` (`self.CounterTop`) 0 "/Game/StarterContent/Materials/M_Rock_Marble_Polished.M_Rock_Marble_Polished"))
    (:`then_1`
      (`PrimitiveComponent.SetMaterial` (`self.CounterElement`) 0 "/Game/CounterWoodNormal.CounterWoodNormal"))))

(fn `CheckIfReferencesAreEqual`
  (params (A :type "Object Object Reference") (B :type "Object Object Reference"))
  (if (== A B)
    _))

(fn `UserConstructionScript`)