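; Onion counter that spawns an OnionBP when X is pressed, at a hardcoded transform rather than one relative to the counter.
; OnInteract swaps in highlight materials when interaction is allowed, and enables player 0's input if the ThirdPersonCharacter carries nothing.
; Tick restores normal materials and disables input every frame, so both states last only while OnInteract keeps firing.
; Overlap helper graphs are present but unused by the event graph.
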(event `Key|X`
  (params (Key :type "Key Structure"))
  (:`Pressed`
    (`|SpawnActorFromClass` "/Game/OnionBP.OnionBP_C" (`KismetMathLibrary.MakeTransform` (0.0 0.0 350.0) (struct) (1.4 1.4 1.2)) "Undefined" "OverrideRootScale" null null)))

(event `/Game/InteractionInterface.OnInteract`
  (params (canCharacterInteract :type Boolean) (interactActor :type "Actor Object Reference"))
  (if canCharacterInteract
    (`|ExecutionSequence`
      (:`then_0`
        (`PrimitiveComponent.SetMaterial` (`self.CounterTop`) 0 "/Game/OnionMaterialOverlap.OnionMaterialOverlap"))
      (:`then_1`
        (`PrimitiveComponent.SetMaterial` (`self.CounterElement`) 0 "/Game/CounterWoodOverlap.CounterWoodOverlap"))
      (:`then_2`
        (bind _asthird_person_character (cast `/Game/ThirdPersonBP/Blueprints/ThirdPersonCharacter` interactActor))
        (if (not (`/Game/ThirdPersonBP/Blueprints/ThirdPersonCharacter.isCarrying` _asthird_person_character))
          (`self.EnableInput` (`GameplayStatics.GetPlayerController` 0)))))))

(event `self.ReceiveTick`
  (params (DeltaSeconds :type "Float (single-precision)"))
  (`|ExecutionSequence`
    (:`then_0`
      (`PrimitiveComponent.SetMaterial` (`self.CounterTop`) 0 "/Game/OnionMaterial.OnionMaterial"))
    (:`then_1`
      (`PrimitiveComponent.SetMaterial` (`self.CounterElement`) 0 "/Game/CounterWoodNormal.CounterWoodNormal"))
    (:`then_2`
      (`self.DisableInput` (`GameplayStatics.GetPlayerController` 0)))))

(fn `CheckIfReferencesAreEqual`
  (params (A :type "Object Object Reference") (B :type "Object Object Reference"))
  (if (== A B)
    _))

(fn `isSomethingPlacedOnElement`
  (returns (isSomethingPlaced :type Boolean))
  (return false))

(fn `UserConstructionScript`)